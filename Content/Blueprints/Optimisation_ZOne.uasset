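; Optimisation zone actor for one cell of a 5x5 tagged grid (A1–E5), hiding content in selected cells.
; ON/OFF events set HideMeActivate on the matching zone, driven by a 25-entry ActivatorArray.
; UpdateHidden then hides or shows "Optimize"-tagged actors overlapping each zone's Box, which is sized in the construction script.
; The per-cell visibility presets are disconnected, and the begin-overlap event is empty, so nothing here triggers the culling.
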(event `E1_ON`
  ;[1 1 1] E Actions
  (bind _outactors (`GameplayStatics.GetAllActorsWithTag` "E1"))
  (bind _asoptimisation_zone (cast `/Game/Blueprints/Optimisation_ZOne` (`KismetArrayLibrary.Array_Get` _outactors)))
  (set `/Game/Blueprints/Optimisation_ZOne.HideMeActivate` true _asoptimisation_zone))

(event `D1_ON`
  ;[1 1 1] D Actions
  (bind _outactors (`GameplayStatics.GetAllActorsWithTag` "D1"))
  (bind _asoptimisation_zone (cast `/Game/Blueprints/Optimisation_ZOne` (`KismetArrayLibrary.Array_Get` _outactors)))
  (set `/Game/Blueprints/Optimisation_ZOne.HideMeActivate` true _asoptimisation_zone))

(event `A1_ON`
  ;[1 1 1] A Actions
  (bind _outactors (`GameplayStatics.GetAllActorsWithTag` "A1"))
  (bind _asoptimisation_zone (cast `/Game/Blueprints/Optimisation_ZOne` (`KismetArrayLibrary.Array_Get` _outactors)))
  (set `/Game/Blueprints/Optimisation_ZOne.HideMeActivate` true _asoptimisation_zone))

(event `B1_ON`
  ;[1 1 1] B Actions
  (bind _outactors (`GameplayStatics.GetAllActorsWithTag` "B1"))
  (bind _asoptimisation_zone (cast `/Game/Blueprints/Optimisation_ZOne` (`KismetArrayLibrary.Array_Get` _outactors)))
  (set `/Game/Blueprints/Optimisation_ZOne.HideMeActivate` true _asoptimisation_zone))

(event `C1_ON`
  ;[1 1 1] C Actions
  (bind _outactors (`GameplayStatics.GetAllActorsWithTag` "C1"))
  (bind _asoptimisation_zone (cast `/Game/Blueprints/Optimisation_ZOne` (`KismetArrayLibrary.Array_Get` _outactors)))
  (set `/Game/Blueprints/Optimisation_ZOne.HideMeActivate` true _asoptimisation_zone))

(event `E1_OFF`
  ;[1 1 1] E Actions
  (bind _outactors (`GameplayStatics.GetAllActorsWithTag` "E1"))
  (bind _asoptimisation_zone (cast `/Game/Blueprints/Optimisation_ZOne` (`KismetArrayLibrary.Array_Get` _outactors)))
  (set `/Game/Blueprints/Optimisation_ZOne.HideMeActivate` false _asoptimisation_zone))

(event `D1_OFF`
  ;[1 1 1] D Actions
  (bind _outactors (`GameplayStatics.GetAllActorsWithTag` "D1"))
  (bind _asoptimisation_zone (cast `/Game/Blueprints/Optimisation_ZOne` (`KismetArrayLibrary.Array_Get` _outactors)))
  (set `/Game/Blueprints/Optimisation_ZOne.HideMeActivate` false _asoptimisation_zone))

(event `A1_OFF`
  ;[1 1 1] A Actions
  (bind _outactors (`GameplayStatics.GetAllActorsWithTag` "A1"))
  (bind _asoptimisation_zone (cast `/Game/Blueprints/Optimisation_ZOne` (`KismetArrayLibrary.Array_Get` _outactors)))
  (set `/Game/Blueprints/Optimisation_ZOne.HideMeActivate` false _asoptimisation_zone))

(event `B1_OFF`
  ;[1 1 1] B Actions
  (bind _outactors (`GameplayStatics.GetAllActorsWithTag` "B1"))
  (bind _asoptimisation_zone (cast `/Game/Blueprints/Optimisation_ZOne` (`KismetArrayLibrary.Array_Get` _outactors)))
  (set `/Game/Blueprints/Optimisation_ZOne.HideMeActivate` false _asoptimisation_zone))

(event `C1_OFF`
  ;[1 1 1] C Actions
  (bind _outactors (`GameplayStatics.GetAllActorsWithTag` "C1"))
  (bind _asoptimisation_zone (cast `/Game/Blueprints/Optimisation_ZOne` (`KismetArrayLibrary.Array_Get` _outactors)))
  (set `/Game/Blueprints/Optimisation_ZOne.HideMeActivate` false _asoptimisation_zone))

(event `E2_ON`
  ;[1 1 1] E Actions
  (bind _outactors (`GameplayStatics.GetAllActorsWithTag` "E2"))
  (bind _asoptimisation_zone (cast `/Game/Blueprints/Optimisation_ZOne` (`KismetArrayLibrary.Array_Get` _outactors)))
  (set `/Game/Blueprints/Optimisation_ZOne.HideMeActivate` true _asoptimisation_zone))

(event `D2_ON`
  ;[1 1 1] D Actions
  (bind _outactors (`GameplayStatics.GetAllActorsWithTag` "D2"))
  (bind _asoptimisation_zone (cast `/Game/Blueprints/Optimisation_ZOne` (`KismetArrayLibrary.Array_Get` _outactors)))
  (set `/Game/Blueprints/Optimisation_ZOne.HideMeActivate` true _asoptimisation_zone))

(event `A2_ON`
  ;[1 1 1] A Actions
  (bind _outactors (`GameplayStatics.GetAllActorsWithTag` "A2"))
  (bind _asoptimisation_zone (cast `/Game/Blueprints/Optimisation_ZOne` (`KismetArrayLibrary.Array_Get` _outactors)))
  (set `/Game/Blueprints/Optimisation_ZOne.HideMeActivate` true _asoptimisation_zone))

(event `B2_ON`
  ;[1 1 1] B Actions
  (bind _outactors (`GameplayStatics.GetAllActorsWithTag` "B2"))
  (bind _asoptimisation_zone (cast `/Game/Blueprints/Optimisation_ZOne` (`KismetArrayLibrary.Array_Get` _outactors)))
  (set `/Game/Blueprints/Optimisation_ZOne.HideMeActivate` true _asoptimisation_zone))

(event `C2_ON`
  ;[1 1 1] C Actions
  (bind _outactors (`GameplayStatics.GetAllActorsWithTag` "C2"))
  (bind _asoptimisation_zone (cast `/Game/Blueprints/Optimisation_ZOne` (`KismetArrayLibrary.Array_Get` _outactors)))
  (set `/Game/Blueprints/Optimisation_ZOne.HideMeActivate` true _asoptimisation_zone))

(event `E2_OFF`
  ;[1 1 1] E Actions
  (bind _outactors (`GameplayStatics.GetAllActorsWithTag` "E2"))
  (bind _asoptimisation_zone (cast `/Game/Blueprints/Optimisation_ZOne` (`KismetArrayLibrary.Array_Get` _outactors)))
  (set `/Game/Blueprints/Optimisation_ZOne.HideMeActivate` false _asoptimisation_zone))

(event `D2_OFF`
  ;[1 1 1] D Actions
  (bind _outactors (`GameplayStatics.GetAllActorsWithTag` "D2"))
  (bind _asoptimisation_zone (cast `/Game/Blueprints/Optimisation_ZOne` (`KismetArrayLibrary.Array_Get` _outactors)))
  (set `/Game/Blueprints/Optimisation_ZOne.HideMeActivate` false _asoptimisation_zone))

(event `A2_OFF`
  ;[1 1 1] A Actions
  (bind _outactors (`GameplayStatics.GetAllActorsWithTag` "A2"))
  (bind _asoptimisation_zone (cast `/Game/Blueprints/Optimisation_ZOne` (`KismetArrayLibrary.Array_Get` _outactors)))
  (set `/Game/Blueprints/Optimisation_ZOne.HideMeActivate` false _asoptimisation_zone))

(event `B2_OFF`
  ;[1 1 1] B Actions
  (bind _outactors (`GameplayStatics.GetAllActorsWithTag` "B2"))
  (bind _asoptimisation_zone (cast `/Game/Blueprints/Optimisation_ZOne` (`KismetArrayLibrary.Array_Get` _outactors)))
  (set `/Game/Blueprints/Optimisation_ZOne.HideMeActivate` false _asoptimisation_zone))

(event `C2_OFF`
  ;[1 1 1] C Actions
  (bind _outactors (`GameplayStatics.GetAllActorsWithTag` "C2"))
  (bind _asoptimisation_zone (cast `/Game/Blueprints/Optimisation_ZOne` (`KismetArrayLibrary.Array_Get` _outactors)))
  (set `/Game/Blueprints/Optimisation_ZOne.HideMeActivate` false _asoptimisation_zone))

(event `E3_ON`
  ;[1 1 1] E Actions
  (bind _outactors (`GameplayStatics.GetAllActorsWithTag` "E3"))
  (bind _asoptimisation_zone (cast `/Game/Blueprints/Optimisation_ZOne` (`KismetArrayLibrary.Array_Get` _outactors)))
  (set `/Game/Blueprints/Optimisation_ZOne.HideMeActivate` true _asoptimisation_zone))

(event `D3_ON`
  ;[1 1 1] D Actions
  (bind _outactors (`GameplayStatics.GetAllActorsWithTag` "D3"))
  (bind _asoptimisation_zone (cast `/Game/Blueprints/Optimisation_ZOne` (`KismetArrayLibrary.Array_Get` _outactors)))
  (set `/Game/Blueprints/Optimisation_ZOne.HideMeActivate` true _asoptimisation_zone))

(event `A3_ON`
  ;[1 1 1] A Actions
  (bind _outactors (`GameplayStatics.GetAllActorsWithTag` "A3"))
  (bind _asoptimisation_zone (cast `/Game/Blueprints/Optimisation_ZOne` (`KismetArrayLibrary.Array_Get` _outactors)))
  (set `/Game/Blueprints/Optimisation_ZOne.HideMeActivate` true _asoptimisation_zone))

(event `B3_ON`
  ;[1 1 1] B Actions
  (bind _outactors (`GameplayStatics.GetAllActorsWithTag` "B3"))
  (bind _asoptimisation_zone (cast `/Game/Blueprints/Optimisation_ZOne` (`KismetArrayLibrary.Array_Get` _outactors)))
  (set `/Game/Blueprints/Optimisation_ZOne.HideMeActivate` true _asoptimisation_zone))

(event `C3_ON`
  ;[1 1 1] C Actions
  (bind _outactors (`GameplayStatics.GetAllActorsWithTag` "C3"))
  (bind _asoptimisation_zone (cast `/Game/Blueprints/Optimisation_ZOne` (`KismetArrayLibrary.Array_Get` _outactors)))
  (set `/Game/Blueprints/Optimisation_ZOne.HideMeActivate` true _asoptimisation_zone))

(event `E3_OFF`
  ;[1 1 1] E Actions
  (bind _outactors (`GameplayStatics.GetAllActorsWithTag` "E3"))
  (bind _asoptimisation_zone (cast `/Game/Blueprints/Optimisation_ZOne` (`KismetArrayLibrary.Array_Get` _outactors)))
  (set `/Game/Blueprints/Optimisation_ZOne.HideMeActivate` false _asoptimisation_zone))

(event `D3_OFF`
  ;[1 1 1] D Actions
  (bind _outactors (`GameplayStatics.GetAllActorsWithTag` "D3"))
  (bind _asoptimisation_zone (cast `/Game/Blueprints/Optimisation_ZOne` (`KismetArrayLibrary.Array_Get` _outactors)))
  (set `/Game/Blueprints/Optimisation_ZOne.HideMeActivate` false _asoptimisation_zone))

(event `A3_OFF`
  ;[1 1 1] A Actions
  (bind _outactors (`GameplayStatics.GetAllActorsWithTag` "A3"))
  (bind _asoptimisation_zone (cast `/Game/Blueprints/Optimisation_ZOne` (`KismetArrayLibrary.Array_Get` _outactors)))
  (set `/Game/Blueprints/Optimisation_ZOne.HideMeActivate` false _asoptimisation_zone))

(event `B3_OFF`
  ;[1 1 1] B Actions
  (bind _outactors (`GameplayStatics.GetAllActorsWithTag` "B3"))
  (bind _asoptimisation_zone (cast `/Game/Blueprints/Optimisation_ZOne` (`KismetArrayLibrary.Array_Get` _outactors)))
  (set `/Game/Blueprints/Optimisation_ZOne.HideMeActivate` false _asoptimisation_zone))

(event `C3_OFF`
  ;[1 1 1] C Actions
  (bind _outactors (`GameplayStatics.GetAllActorsWithTag` "C3"))
  (bind _asoptimisation_zone (cast `/Game/Blueprints/Optimisation_ZOne` (`KismetArrayLibrary.Array_Get` _outactors)))
  (set `/Game/Blueprints/Optimisation_ZOne.HideMeActivate` false _asoptimisation_zone))

(event `E4_ON`
  ;[1 1 1] E Actions
  (bind _outactors (`GameplayStatics.GetAllActorsWithTag` "E4"))
  (bind _asoptimisation_zone (cast `/Game/Blueprints/Optimisation_ZOne` (`KismetArrayLibrary.Array_Get` _outactors)))
  (set `/Game/Blueprints/Optimisation_ZOne.HideMeActivate` true _asoptimisation_zone))

(event `D4_ON`
  ;[1 1 1] D Actions
  (bind _outactors (`GameplayStatics.GetAllActorsWithTag` "D4"))
  (bind _asoptimisation_zone (cast `/Game/Blueprints/Optimisation_ZOne` (`KismetArrayLibrary.Array_Get` _outactors)))
  (set `/Game/Blueprints/Optimisation_ZOne.HideMeActivate` true _asoptimisation_zone))

(event `A4_ON`
  ;[1 1 1] A Actions
  (bind _outactors (`GameplayStatics.GetAllActorsWithTag` "A4"))
  (bind _asoptimisation_zone (cast `/Game/Blueprints/Optimisation_ZOne` (`KismetArrayLibrary.Array_Get` _outactors)))
  (set `/Game/Blueprints/Optimisation_ZOne.HideMeActivate` true _asoptimisation_zone))

(event `B4_ON`
  ;[1 1 1] B Actions
  (bind _outactors (`GameplayStatics.GetAllActorsWithTag` "B4"))
  (bind _asoptimisation_zone (cast `/Game/Blueprints/Optimisation_ZOne` (`KismetArrayLibrary.Array_Get` _outactors)))
  (set `/Game/Blueprints/Optimisation_ZOne.HideMeActivate` true _asoptimisation_zone))

(event `C4_ON`
  ;[1 1 1] C Actions
  (bind _outactors (`GameplayStatics.GetAllActorsWithTag` "C4"))
  (bind _asoptimisation_zone (cast `/Game/Blueprints/Optimisation_ZOne` (`KismetArrayLibrary.Array_Get` _outactors)))
  (set `/Game/Blueprints/Optimisation_ZOne.HideMeActivate` true _asoptimisation_zone))

(event `E4_OFF`
  ;[1 1 1] E Actions
  (bind _outactors (`GameplayStatics.GetAllActorsWithTag` "E4"))
  (bind _asoptimisation_zone (cast `/Game/Blueprints/Optimisation_ZOne` (`KismetArrayLibrary.Array_Get` _outactors)))
  (set `/Game/Blueprints/Optimisation_ZOne.HideMeActivate` false _asoptimisation_zone))

(event `D4_OFF`
  ;[1 1 1] D Actions
  (bind _outactors (`GameplayStatics.GetAllActorsWithTag` "D4"))
  (bind _asoptimisation_zone (cast `/Game/Blueprints/Optimisation_ZOne` (`KismetArrayLibrary.Array_Get` _outactors)))
  (set `/Game/Blueprints/Optimisation_ZOne.HideMeActivate` false _asoptimisation_zone))

(event `A4_OFF`
  ;[1 1 1] A Actions
  (bind _outactors (`GameplayStatics.GetAllActorsWithTag` "A4"))
  (bind _asoptimisation_zone (cast `/Game/Blueprints/Optimisation_ZOne` (`KismetArrayLibrary.Array_Get` _outactors)))
  (set `/Game/Blueprints/Optimisation_ZOne.HideMeActivate` false _asoptimisation_zone))

(event `B4_OFF`
  ;[1 1 1] B Actions
  (bind _outactors (`GameplayStatics.GetAllActorsWithTag` "B4"))
  (bind _asoptimisation_zone (cast `/Game/Blueprints/Optimisation_ZOne` (`KismetArrayLibrary.Array_Get` _outactors)))
  (set `/Game/Blueprints/Optimisation_ZOne.HideMeActivate` false _asoptimisation_zone))

(event `C4_OFF`
  ;[1 1 1] C Actions
  (bind _outactors (`GameplayStatics.GetAllActorsWithTag` "C4"))
  (bind _asoptimisation_zone (cast `/Game/Blueprints/Optimisation_ZOne` (`KismetArrayLibrary.Array_Get` _outactors)))
  (set `/Game/Blueprints/Optimisation_ZOne.HideMeActivate` false _asoptimisation_zone))

(event `E5_ON`
  ;[1 1 1] E Actions
  (bind _outactors (`GameplayStatics.GetAllActorsWithTag` "E5"))
  (bind _asoptimisation_zone (cast `/Game/Blueprints/Optimisation_ZOne` (`KismetArrayLibrary.Array_Get` _outactors)))
  (set `/Game/Blueprints/Optimisation_ZOne.HideMeActivate` true _asoptimisation_zone))

(event `D5_ON`
  ;[1 1 1] D Actions
  (bind _outactors (`GameplayStatics.GetAllActorsWithTag` "D5"))
  (bind _asoptimisation_zone (cast `/Game/Blueprints/Optimisation_ZOne` (`KismetArrayLibrary.Array_Get` _outactors)))
  (set `/Game/Blueprints/Optimisation_ZOne.HideMeActivate` true _asoptimisation_zone))

(event `A5_ON`
  ;[1 1 1] A Actions
  (bind _outactors (`GameplayStatics.GetAllActorsWithTag` "A5"))
  (bind _asoptimisation_zone (cast `/Game/Blueprints/Optimisation_ZOne` (`KismetArrayLibrary.Array_Get` _outactors)))
  (set `/Game/Blueprints/Optimisation_ZOne.HideMeActivate` true _asoptimisation_zone))

(event `B5_ON`
  ;[1 1 1] B Actions
  (bind _outactors (`GameplayStatics.GetAllActorsWithTag` "B5"))
  (bind _asoptimisation_zone (cast `/Game/Blueprints/Optimisation_ZOne` (`KismetArrayLibrary.Array_Get` _outactors)))
  (set `/Game/Blueprints/Optimisation_ZOne.HideMeActivate` true _asoptimisation_zone))

(event `C5_ON`
  ;[1 1 1] C Actions
  (bind _outactors (`GameplayStatics.GetAllActorsWithTag` "C5"))
  (bind _asoptimisation_zone (cast `/Game/Blueprints/Optimisation_ZOne` (`KismetArrayLibrary.Array_Get` _outactors)))
  (set `/Game/Blueprints/Optimisation_ZOne.HideMeActivate` true _asoptimisation_zone))

(event `E5_OFF`
  ;[1 1 1] E Actions
  (bind _outactors (`GameplayStatics.GetAllActorsWithTag` "E5"))
  (bind _asoptimisation_zone (cast `/Game/Blueprints/Optimisation_ZOne` (`KismetArrayLibrary.Array_Get` _outactors)))
  (set `/Game/Blueprints/Optimisation_ZOne.HideMeActivate` false _asoptimisation_zone))

(event `D5_OFF`
  ;[1 1 1] D Actions
  (bind _outactors (`GameplayStatics.GetAllActorsWithTag` "D5"))
  (bind _asoptimisation_zone (cast `/Game/Blueprints/Optimisation_ZOne` (`KismetArrayLibrary.Array_Get` _outactors)))
  (set `/Game/Blueprints/Optimisation_ZOne.HideMeActivate` false _asoptimisation_zone))

(event `A5_OFF`
  ;[1 1 1] A Actions
  (bind _outactors (`GameplayStatics.GetAllActorsWithTag` "A5"))
  (bind _asoptimisation_zone (cast `/Game/Blueprints/Optimisation_ZOne` (`KismetArrayLibrary.Array_Get` _outactors)))
  (set `/Game/Blueprints/Optimisation_ZOne.HideMeActivate` false _asoptimisation_zone))

(event `B5_OFF`
  ;[1 1 1] B Actions
  (bind _outactors (`GameplayStatics.GetAllActorsWithTag` "B5"))
  (bind _asoptimisation_zone (cast `/Game/Blueprints/Optimisation_ZOne` (`KismetArrayLibrary.Array_Get` _outactors)))
  (set `/Game/Blueprints/Optimisation_ZOne.HideMeActivate` false _asoptimisation_zone))

(event `C5_OFF`
  ;[1 1 1] C Actions
  (bind _outactors (`GameplayStatics.GetAllActorsWithTag` "C5"))
  (bind _asoptimisation_zone (cast `/Game/Blueprints/Optimisation_ZOne` (`KismetArrayLibrary.Array_Get` _outactors)))
  (set `/Game/Blueprints/Optimisation_ZOne.HideMeActivate` false _asoptimisation_zone))

(event `ResetAll`
  (`self.A1_OFF`)
  (`self.A2_OFF`)
  (`self.A3_OFF`)
  (`self.A4_OFF`)
  (`self.A5_OFF`)
  (`self.B5_OFF`)
  (`self.B4_OFF`)
  (`self.B3_OFF`)
  (`self.B2_OFF`)
  (`self.B1_OFF`)
  (`self.C1_OFF`)
  (`self.C2_OFF`)
  (`self.C3_OFF`)
  (`self.C4_OFF`)
  (`self.C5_OFF`)
  (`self.D5_OFF`)
  (`self.D4_OFF`)
  (`self.D3_OFF`)
  (`self.D2_OFF`)
  (`self.D1_OFF`)
  (`self.E1_OFF`)
  (`self.E2_OFF`)
  (`self.E3_OFF`)
  (`self.E4_OFF`)
  (`self.E5_OFF`))

(event `CheckActivatorArray`
  (for (_array_element _array_index) (`self.ActivatorArray`)
    (if _array_element
      (switch `int` _array_index
        (:`0`
          (`self.A1_ON`))
        (:`1`
          (`self.A2_ON`))
        (:`2`
          (`self.A3_ON`))
        (:`3`
          (`self.A4_ON`))
        (:`4`
          (`self.A5_ON`))
        (:`5`
          (`self.B1_ON`))
        (:`6`
          (`self.B2_ON`))
        (:`7`
          (`self.B3_ON`))
        (:`8`
          (`self.B4_ON`))
        (:`9`
          (`self.B5_ON`))
        (:`10`
          (`self.C1_ON`))
        (:`11`
          (`self.C2_ON`))
        (:`12`
          (`self.C3_ON`))
        (:`13`
          (`self.C4_ON`))
        (:`14`
          (`self.C5_ON`))
        (:`15`
          (`self.D1_ON`))
        (:`16`
          (`self.D2_ON`))
        (:`17`
          (`self.D3_ON`))
        (:`18`
          (`self.D4_ON`))
        (:`19`
          (`self.D5_ON`))
        (:`20`
          (`self.E1_ON`))
        (:`21`
          (`self.E2_ON`))
        (:`22`
          (`self.E3_ON`))
        (:`23`
          (`self.E4_ON`))
        (:`24`
          (`self.E5_ON`)))))
  (`self.UpdateHidden`))

(event `UpdateHidden`
  (bind _outactors (`GameplayStatics.GetAllActorsOfClass` "Optimisation_Zone_C"))
  (for _array_element _outactors
    (if (`/Game/Blueprints/Optimisation_ZOne.HideMeActivate` _array_element)
      (bind _outactors_2 (`GameplayStatics.GetAllActorsWithTag` "Optimize"))
      (for _array_element_2 _outactors_2
        (bind _box (`/Game/Blueprints/Optimisation_ZOne.Box` _array_element))
        (if (`PrimitiveComponent.IsOverlappingActor` _box _array_element_2)
          (`self.SetActorHiddenInGame` _array_element_2 true)))
      (else
        (bind _outactors_3 (`GameplayStatics.GetAllActorsWithTag` "Optimize"))
        (for _array_element_3 _outactors_3
          (if (`PrimitiveComponent.IsOverlappingActor` _box _array_element_3)
            (`self.SetActorHiddenInGame` _array_element_3 false)))))))

(event `self.ReceiveActorBeginOverlap`
  (params (OtherActor :type "Actor Object Reference")))

(fn `UserConstructionScript`
  (`BoxComponent.SetBoxExtent` (`self.Box`) (`KismetMathLibrary.MakeVector` (`self.X`) (`self.Y`) (`self.Z`)) true))