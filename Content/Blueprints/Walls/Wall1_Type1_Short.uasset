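; A short type-1 wall piece Blueprint with a main wall mesh and optional top and bottom stub meshes.
; The construction script applies a wall material to the wall and a shared stub material to both stubs.
; Two boolean variables toggle each stub's visibility and collision together, so hidden stubs do not block anything.
; The event graph holds no runtime logic.
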(event `self.ReceiveBeginPlay`)

(fn `UserConstructionScript`
  (bind _bottom (`self.Bottom`))
  (bind _stub_material (`self.Stub_Material`))
  (bind _staticmesh (`self.StaticMesh`))
  (bind _bottom_2 (`self.Bottom`))
  (bind _staticmesh_2 (`self.StaticMesh`))
  (`PrimitiveComponent.SetMaterial` (`self.Wall`) 0 (`self.Wall_Material`))
  (`PrimitiveComponent.SetMaterial` (`self.StaticMesh`) 0 _stub_material)
  (`PrimitiveComponent.SetMaterial` (`self.Bottom`) 0 _stub_material)
  (`|ExecutionSequence`
    (:`then_0`
      (if (`self.StubBotVisible`)
        (`SceneComponent.SetVisibility` _bottom true false)
        (`PrimitiveComponent.SetCollisionEnabled` _bottom "QueryAndPhysics")
        (else
          (`SceneComponent.SetVisibility` _bottom_2 false false)
          (`PrimitiveComponent.SetCollisionEnabled` _bottom_2 "NoCollision"))))
    (:`then_1`
      (if (`self.StubTopVisible`)
        (`SceneComponent.SetVisibility` _staticmesh true false)
        (`PrimitiveComponent.SetCollisionEnabled` _staticmesh "QueryAndPhysics")
        (else
          (`SceneComponent.SetVisibility` _staticmesh_2 false false)
          (`PrimitiveComponent.SetCollisionEnabled` _staticmesh_2 "NoCollision"))))))