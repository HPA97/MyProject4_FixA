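; Wall piece with a double-door opening whose two doors are physics-simulated on the authority and have physics disabled on remote machines.
; Each tick, the authority stores both doors' relative transforms, while remotes apply the stored transformation variables to the doors as world transforms.
; The construction script assigns configurable materials to the wall's front and back, both doors and both stubs.
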(event `self.ReceiveBeginPlay`
  (bind _door (`self.Door`))
  (bind _door2 (`self.Door2`))
  (`/Engine/EditorBlueprintResources/ActorMacros.Switch Has Authority`
    (:`Authority`
      (`PrimitiveComponent.SetSimulatePhysics` _door true)
      (set `self.Transformation` (`SceneComponent.GetRelativeTransform` (`self.Door`)))
      (`PrimitiveComponent.SetSimulatePhysics` _door2 true)
      (set `self.Transformation2` (`SceneComponent.GetRelativeTransform` (`self.Door2`))))
    (:`Remote`
      (`PrimitiveComponent.SetSimulatePhysics` _door false)
      (`PrimitiveComponent.SetSimulatePhysics` _door2 false))))

(event `self.ReceiveTick`
  (params (DeltaSeconds :type "Float (single-precision)"))
  (`self.UpdateRotation`))

(event `UpdateRotation`
  (bind _door (`self.Door`))
  (bind _door2 (`self.Door2`))
  (`/Engine/EditorBlueprintResources/ActorMacros.Switch Has Authority`
    (:`Authority`
      (set `self.Transformation` (`SceneComponent.GetRelativeTransform` _door))
      (set `self.Transformation2` (`SceneComponent.GetRelativeTransform` _door2)))
    (:`Remote`
      (`SceneComponent.K2_SetWorldTransform` _door (`self.Transformation`) false false)
      (`SceneComponent.K2_SetWorldTransform` _door2 (`self.Transformation2`) false false))))

(fn `UserConstructionScript`
  (bind _wall (`self.Wall`))
  (bind _stub_material (`self.Stub_Material`))
  (`PrimitiveComponent.SetMaterial` _wall 0 (`self.Wall_Front_Material`))
  (`PrimitiveComponent.SetMaterial` _wall 2 (`self.Wall_Back_Material`))
  (`PrimitiveComponent.SetMaterial` (`self.Door`) 0 (`self.Door_Material`))
  (`PrimitiveComponent.SetMaterial` (`self.Door2`) 0 (`self.Door_Material`))
  (`PrimitiveComponent.SetMaterial` (`self.Stub`) 0 _stub_material)
  (`PrimitiveComponent.SetMaterial` (`self.Stub2`) 0 _stub_material))