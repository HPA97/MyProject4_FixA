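; Wall1_Type1_Window_02 is a modular wall piece Blueprint, named as a window variant, with configurable materials.
; Its construction script applies front, back and frame material variables to separate slots of the Wall mesh.
; Two further static mesh components share a stub material.
; The event graph holds only empty default events, so the Blueprint adds no runtime logic.
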(event `self.ReceiveBeginPlay`)

(fn `UserConstructionScript`
  (bind _stub_material (`self.Stub_Material`))
  (bind _wall (`self.Wall`))
  (`PrimitiveComponent.SetMaterial` _wall 0 (`self.Wall_Front_Material`))
  (`PrimitiveComponent.SetMaterial` (`self.StaticMesh1`) 0 _stub_material)
  (`PrimitiveComponent.SetMaterial` (`self.StaticMesh`) 0 _stub_material)
  (`PrimitiveComponent.SetMaterial` _wall 2 (`self.Wall_Back_Material`))
  (`PrimitiveComponent.SetMaterial` _wall 3 (`self.Frame_Material`)))