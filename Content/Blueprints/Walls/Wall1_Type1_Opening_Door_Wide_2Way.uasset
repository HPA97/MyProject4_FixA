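; Wall segment Blueprint with a wide opening door, which swings by physics simulation on the authority only.
; Each Tick the authority stores the door's relative transform in Transformation, while remotes, with physics disabled, apply that variable to the door as a world transform.
; The construction script assigns configurable materials to the wall's front, back and frame slots and to the door.
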(event `self.ReceiveBeginPlay`
  (bind _door (`self.Door`))
  (`/Engine/EditorBlueprintResources/ActorMacros.Switch Has Authority`
    (:`Authority`
      (`PrimitiveComponent.SetSimulatePhysics` _door true)
      (set `self.Transformation` (`SceneComponent.GetRelativeTransform` (`self.Door`))))
    (:`Remote`
      (`PrimitiveComponent.SetSimulatePhysics` _door false))))

(event `self.ReceiveTick`
  (params (DeltaSeconds :type "Float (single-precision)"))
  (`self.UpdateRotation`))

(event `UpdateRotation`
  (bind _door (`self.Door`))
  (`/Engine/EditorBlueprintResources/ActorMacros.Switch Has Authority`
    (:`Authority`
      (set `self.Transformation` (`SceneComponent.GetRelativeTransform` _door)))
    (:`Remote`
      (`SceneComponent.K2_SetWorldTransform` _door (`self.Transformation`) false false))))

(fn `UserConstructionScript`
  (bind _wall (`self.Wall`))
  (`PrimitiveComponent.SetMaterial` _wall 0 (`self.Wall_Front_Material`))
  (`PrimitiveComponent.SetMaterial` _wall 4 (`self.Frame_Material`))
  (`PrimitiveComponent.SetMaterial` _wall 3 (`self.Wall_Back_Material`))
  (`PrimitiveComponent.SetMaterial` (`self.Door`) 0 (`self.Door_Material`)))