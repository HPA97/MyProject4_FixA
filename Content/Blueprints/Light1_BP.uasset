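; Light1_BP is a point light actor with per-instance color and visibility, applied in the Construction Script.
; Its Event Graph holds unreachable logic for an F-key light toggle and player detection that switches input and prompt text visibility.
; None of that logic is hooked to a live event, so only the construction-time setup takes effect.
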(fn `UserConstructionScript`
  (bind _pointlight (`self.PointLight`))
  (`LightComponent.SetLightColor` _pointlight (`self.Light Color`) true)
  (`SceneComponent.SetVisibility` _pointlight (`self.Visibility Setting`) false))