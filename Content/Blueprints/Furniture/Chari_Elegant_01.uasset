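; Elegant chair furniture Blueprint with configurable materials for each part of its mesh.
; The construction script assigns four material variables to the Chair component's slots: bottom, cushion, middle frame and back part.
; The event graph holds only disabled placeholder events, so the chair has no runtime logic.
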(fn `UserConstructionScript`
  (`PrimitiveComponent.SetMaterial` (`self.Chair`) 0 (`self.Material_Bottom`))
  (`PrimitiveComponent.SetMaterial` (`self.Chair`) 1 (`self.Material_Cush`))
  (`PrimitiveComponent.SetMaterial` (`self.Chair`) 2 (`self.Material_Frame_Middle`))
  (`PrimitiveComponent.SetMaterial` (`self.Chair`) 3 (`self.Material_Back_Part`)))