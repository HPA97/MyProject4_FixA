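; Toilet furniture Blueprint with a Plate component that is physics-simulated on the network authority only.
; Every tick, the authority stores the plate's relative transform in Transformation, while remote instances apply that variable to their non-simulated plate as a world transform.
; The construction script assigns separate configurable materials to the Toilet and Plate components.
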(event `self.ReceiveBeginPlay`
  (bind _plate (`self.Plate`))
  (`/Engine/EditorBlueprintResources/ActorMacros.Switch Has Authority`
    (:`Authority`
      (`PrimitiveComponent.SetSimulatePhysics` _plate true)
      (set `self.Transformation` (`SceneComponent.GetRelativeTransform` (`self.Plate`))))
    (:`Remote`
      (`PrimitiveComponent.SetSimulatePhysics` _plate false))))

(event `self.ReceiveTick`
  (params (DeltaSeconds :type "Float (single-precision)"))
  (`self.UpdateRotation`))

(event `UpdateRotation`
  (bind _plate (`self.Plate`))
  (`/Engine/EditorBlueprintResources/ActorMacros.Switch Has Authority`
    (:`Authority`
      (set `self.Transformation` (`SceneComponent.GetRelativeTransform` _plate)))
    (:`Remote`
      (`SceneComponent.K2_SetWorldTransform` _plate (`self.Transformation`) false false))))

(fn `UserConstructionScript`
  (`PrimitiveComponent.SetMaterial` (`self.Toilet`) 0 (`self.Material_Main`))
  (`PrimitiveComponent.SetMaterial` (`self.Plate`) 0 (`self.Material_Plate`)))