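; StarStep1 is a step prop actor with a selectable carpet material.
; The construction script compares MaterialTopType against five options and applies the matching carpet material instance to element 0 of its StaticMesh.
; Values outside those options leave the material untouched, and the event graph holds no runtime logic.
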(fn `UserConstructionScript`
  (`|ExecutionSequence`
    (:`then_0`
      (if (== (`self.MaterialTopType`) 0)
        (`PrimitiveComponent.SetMaterial` (`self.StaticMesh`) 0 "/Game/Materials/Carpet3_Inst.Carpet3_Inst")))
    (:`then_1`
      (if (== (`self.MaterialTopType`) 1)
        (`PrimitiveComponent.SetMaterial` (`self.StaticMesh`) 0 "/Game/Materials/Carpet4_Inst.Carpet4_Inst")))
    (:`then_2`
      (if (== (`self.MaterialTopType`) 2)
        (`PrimitiveComponent.SetMaterial` (`self.StaticMesh`) 0 "/Game/Materials/Carpet2_Inst.Carpet2_Inst")))
    (:`then_3`
      (if (== (`self.MaterialTopType`) 3)
        (`PrimitiveComponent.SetMaterial` (`self.StaticMesh`) 0 "/Game/Materials/Carpet5_Inst.Carpet5_Inst")))
    (:`then_4`
      (if (== (`self.MaterialTopType`) 4)
        (`PrimitiveComponent.SetMaterial` (`self.StaticMesh`) 0 "/Game/Materials/Carpet6_Inst.Carpet6_Inst")))))