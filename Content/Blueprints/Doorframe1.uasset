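; Doorframe Blueprint whose Door1 component is a physics-driven door kept in sync between server and clients.
; Only the authority simulates physics on the door, storing its relative transform in Transformation at start and every tick.
; Remotes disable simulation and apply Transformation each tick, though as a world transform rather than a relative one.
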(event `self.ReceiveBeginPlay`
  (bind _door1 (`self.Door1`))
  (`/Engine/EditorBlueprintResources/ActorMacros.Switch Has Authority`
    (:`Authority`
      (`PrimitiveComponent.SetSimulatePhysics` _door1 true)
      (set `self.Transformation` (`SceneComponent.GetRelativeTransform` (`self.Door1`))))
    (:`Remote`
      (`PrimitiveComponent.SetSimulatePhysics` _door1 false))))

(event `self.ReceiveTick`
  (params (DeltaSeconds :type "Float (single-precision)"))
  (`self.UpdateRotation`))

(event `UpdateRotation`
  (bind _door1 (`self.Door1`))
  (`/Engine/EditorBlueprintResources/ActorMacros.Switch Has Authority`
    (:`Authority`
      (set `self.Transformation` (`SceneComponent.GetRelativeTransform` _door1)))
    (:`Remote`
      (`SceneComponent.K2_SetWorldTransform` _door1 (`self.Transformation`) false false))))

(fn `UserConstructionScript`)