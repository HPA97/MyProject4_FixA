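; Milk carton physics prop for a networked game, with its look chosen by MilkType.
; The construction script applies one of two materials to the mesh based on that type.
; Only the authority simulates physics, storing the mesh's relative transform in Transformation every tick.
; Remote instances disable physics and set the mesh's world transform from that variable each tick, a manual sync without sweep or interpolation.
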(event `self.ReceiveBeginPlay`
  (bind _milkcartong (`self.MilkCartong`))
  (`/Engine/EditorBlueprintResources/ActorMacros.Switch Has Authority`
    (:`Authority`
      (`PrimitiveComponent.SetSimulatePhysics` _milkcartong true)
      (set `self.Transformation` (`SceneComponent.GetRelativeTransform` (`self.MilkCartong`))))
    (:`Remote`
      (`PrimitiveComponent.SetSimulatePhysics` _milkcartong false))))

(event `self.ReceiveTick`
  (params (DeltaSeconds :type "Float (single-precision)"))
  (`self.UpdateTransformation`))

(event `UpdateTransformation`
  (bind _milkcartong (`self.MilkCartong`))
  (`/Engine/EditorBlueprintResources/ActorMacros.Switch Has Authority`
    (:`Authority`
      (set `self.Transformation` (`SceneComponent.GetRelativeTransform` _milkcartong)))
    (:`Remote`
      (`SceneComponent.K2_SetWorldTransform` _milkcartong (`self.Transformation`) false false))))

(fn `UserConstructionScript`
  (bind _milkcartong (`self.MilkCartong`))
  (`|ExecutionSequence`
    (:`then_0`
      (if (== (`self.MilkType`) 0)
        (`PrimitiveComponent.SetMaterial` _milkcartong 0 "/Game/Materials/Milk1.Milk1")))
    (:`then_1`
      (if (== (`self.MilkType`) 1)
        (`PrimitiveComponent.SetMaterial` _milkcartong 0 "/Game/Materials/Milk2.Milk2")))))