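; Networked furniture Blueprint with three physics-driven drawers, where only the authority simulates physics.
; Each tick, the authority stores every drawer's relative transform in a variable, while remote instances disable physics and apply those variables to the drawers.
; The variables presumably replicate, though their settings are not shown here.
; Remote instances apply the stored relative transforms as world transforms, so the two spaces differ.
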(event `self.ReceiveBeginPlay`
  (bind _drawer1 (`self.Drawer1`))
  (bind _drawer2 (`self.Drawer2`))
  (bind _drawer3 (`self.Drawer3`))
  (`/Engine/EditorBlueprintResources/ActorMacros.Switch Has Authority`
    (:`Authority`
      ;[1 1 1] Drawer 1
      (`PrimitiveComponent.SetSimulatePhysics` _drawer1 true)
      (set `self.Transformation1` (`SceneComponent.GetRelativeTransform` (`self.Drawer1`)))
      ;[1 1 1] Drawer 2
      (`PrimitiveComponent.SetSimulatePhysics` _drawer2 true)
      (set `self.Transformation2` (`SceneComponent.GetRelativeTransform` (`self.Drawer2`)))
      ;[1 1 1] Drawer 3
      (`PrimitiveComponent.SetSimulatePhysics` _drawer3 true)
      (set `self.Transformation3` (`SceneComponent.GetRelativeTransform` (`self.Drawer3`))))
    (:`Remote`
      (`PrimitiveComponent.SetSimulatePhysics` _drawer1 false)
      (`PrimitiveComponent.SetSimulatePhysics` _drawer2 false)
      (`PrimitiveComponent.SetSimulatePhysics` _drawer3 false))))

(event `self.ReceiveTick`
  (params (DeltaSeconds :type "Float (single-precision)"))
  (`self.UpdateRotation`))

(event `UpdateRotation`
  (bind _drawer3 (`self.Drawer3`))
  (bind _drawer1 (`self.Drawer1`))
  (bind _drawer2 (`self.Drawer2`))
  (`/Engine/EditorBlueprintResources/ActorMacros.Switch Has Authority`
    (:`Authority`
      ;[1 1 1] Drawer 1
      (set `self.Transformation1` (`SceneComponent.GetRelativeTransform` _drawer1))
      ;[1 1 1] Drawer 2
      (set `self.Transformation2` (`SceneComponent.GetRelativeTransform` _drawer2))
      ;[1 1 1] Drawer 3
      (set `self.Transformation3` (`SceneComponent.GetRelativeTransform` _drawer3)))
    (:`Remote`
      (`SceneComponent.K2_SetWorldTransform` _drawer1 (`self.Transformation1`) false false)
      (`SceneComponent.K2_SetWorldTransform` _drawer2 (`self.Transformation2`) false false)
      (`SceneComponent.K2_SetWorldTransform` _drawer3 (`self.Transformation3`) false false))))

(fn `UserConstructionScript`)