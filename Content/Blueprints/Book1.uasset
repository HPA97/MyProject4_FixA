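; Book prop Blueprint whose look is chosen per placed instance.
; The Construction Script checks the Book variable against eight index values and applies the matching material to element 0 of the Books component.
; The event graph holds only disabled default events, so it adds no runtime behavior.
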(fn `UserConstructionScript`
  (`|ExecutionSequence`
    (:`then_0`
      (if (== (`self.Book`) 0)
        (`PrimitiveComponent.SetMaterial` (`self.Books`) 0 "/Game/Materials/Book1.Book1")))
    (:`then_1`
      (if (== (`self.Book`) 1)
        (`PrimitiveComponent.SetMaterial` (`self.Books`) 0 "/Game/Materials/Book2.Book2")))
    (:`then_2`
      (if (== (`self.Book`) 2)
        (`PrimitiveComponent.SetMaterial` (`self.Books`) 0 "/Game/Materials/Book3.Book3")))
    (:`then_3`
      (if (== (`self.Book`) 3)
        (`PrimitiveComponent.SetMaterial` (`self.Books`) 0 "/Game/Materials/Book4.Book4")))
    (:`then_4`
      (if (== (`self.Book`) 4)
        (`PrimitiveComponent.SetMaterial` (`self.Books`) 0 "/Game/Materials/Book5.Book5")))
    (:`then_5`
      (if (== (`self.Book`) 5)
        (`PrimitiveComponent.SetMaterial` (`self.Books`) 0 "/Game/Materials/Book6.Book6")))
    (:`then_6`
      (if (== (`self.Book`) 6)
        (`PrimitiveComponent.SetMaterial` (`self.Books`) 0 "/Game/Materials/Book7.Book7")))
    (:`then_7`
      (if (== (`self.Book`) 7)
        (`PrimitiveComponent.SetMaterial` (`self.Books`) 0 "/Game/Materials/Book8.Book8")))))