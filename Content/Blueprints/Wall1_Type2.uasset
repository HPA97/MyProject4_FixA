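; Wall actor Blueprint that picks its surface material at runtime from a WallTexture setting.
; On BeginPlay, a Sequence compares WallTexture against fixed indices and sets material slot 1 to the matching wood or brick instance.
; The Construction Script is empty, so the choice is applied only when play begins.
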(event `self.ReceiveBeginPlay`
  (`|ExecutionSequence`
    (:`then_0`
      (if (== (`self.WallTexture`) 0)
        (`PrimitiveComponent.SetMaterial` 1 "/Game/Materials/Wood4_White_Inst2.Wood4_White_Inst2")))
    (:`then_1`
      (if (== (`self.WallTexture`) 1)
        (`PrimitiveComponent.SetMaterial` 1 "/Game/Materials/Wood4_LightOrange_Inst.Wood4_LightOrange_Inst")))
    (:`then_2`
      (if (== (`self.WallTexture`) 2)
        (`PrimitiveComponent.SetMaterial` 1 "/Game/Materials/Wood4_LightBrown_Inst2.Wood4_LightBrown_Inst2")))
    (:`then_3`
      (if (== (`self.WallTexture`) 3)
        (`PrimitiveComponent.SetMaterial` 1 "/Game/Materials/Brick1_Inst2.Brick1_Inst2")))))

(fn `UserConstructionScript`)