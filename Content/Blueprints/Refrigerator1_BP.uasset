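; Refrigerator actor with two physics-driven doors, top and bottom, kept in step across a networked game.
; Only the authority simulates door physics, storing each door's transform on BeginPlay and every Tick.
; Remotes disable door simulation and apply the stored transforms each Tick.
; The values are captured as relative transforms but applied as world transforms.
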(event `self.ReceiveBeginPlay`
  (bind _door_bot (`self.Door_Bot`))
  (bind _door_top (`self.Door_Top`))
  (`/Engine/EditorBlueprintResources/ActorMacros.Switch Has Authority`
    (:`Authority`
      ;[1 1 1] Big Door
      (`PrimitiveComponent.SetSimulatePhysics` _door_bot true)
      (set `self.Transformation1` (`SceneComponent.GetRelativeTransform` (`self.Door_Bot`)))
      ;[1 1 1] Small Door
      (`PrimitiveComponent.SetSimulatePhysics` _door_top true)
      (set `self.Transformation2` (`SceneComponent.GetRelativeTransform` (`self.Door_Top`))))
    (:`Remote`
      (`PrimitiveComponent.SetSimulatePhysics` _door_bot false)
      (`PrimitiveComponent.SetSimulatePhysics` _door_top false))))

(event `self.ReceiveTick`
  (params (DeltaSeconds :type "Float (single-precision)"))
  (`self.UpdateRotation`))

(event `UpdateRotation`
  (bind _door_bot (`self.Door_Bot`))
  (bind _door_top (`self.Door_Top`))
  (`/Engine/EditorBlueprintResources/ActorMacros.Switch Has Authority`
    (:`Authority`
      ;[1 1 1] Big Door
      (set `self.Transformation1` (`SceneComponent.GetRelativeTransform` _door_bot))
      ;[1 1 1] Small Door
      (set `self.Transformation2` (`SceneComponent.GetRelativeTransform` _door_top)))
    (:`Remote`
      (`SceneComponent.K2_SetWorldTransform` _door_bot (`self.Transformation1`) false false)
      (`SceneComponent.K2_SetWorldTransform` _door_top (`self.Transformation2`) false false))))

(fn `UserConstructionScript`)