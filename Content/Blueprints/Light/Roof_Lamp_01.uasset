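; Roof lamp actor Blueprint with a point light that is configured per instance.
; The construction script applies the LightColor and VisibilitySetting variables to the light's color and visibility.
; The event graph holds only disconnected remnants of a player-proximity interaction to toggle the light with the F key, so none of it runs.
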(event `Key|F`
  (params (Key :type "Key Structure" :default "AnyKey"))
  ;[1 1 1] When F is pressed
)

(fn `UserConstructionScript`
  (bind _pointlight (`self.PointLight`))
  (`LightComponent.SetLightColor` _pointlight (`self.Light Color`) true)
  (`SceneComponent.SetVisibility` _pointlight (`self.Visibility Setting`) false))